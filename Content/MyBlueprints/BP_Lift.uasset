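; BP_Lift is a multi-floor elevator whose car moves to a requested floor through CallLift, with travel time proportional to floors crossed.
; The construction script stacks instanced shaft, door and floor meshes at GlobalOffset intervals and tags a child BP_Button per floor with its index.
; It then randomizes the car's starting floor using a hardcoded 1000-unit spacing and sets PlayerStartRef's height to 230 plus an unscaled random integer.
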(event `Call Lift`
  (params (FloorIndex :type Integer))
  (bind _liftbase (`self.LiftBase`))
  (bind (_relativelocation_x _relativelocation_y) (`KismetMathLibrary.BreakVector` (`SceneComponent.RelativeLocation` _liftbase)))
  ;[0.07292 0.07292 0.07292] Call Lift
  (if (!= FloorIndex (`self.ActualLiftFloor`))
    (`KismetSystemLibrary.MoveComponentTo` _liftbase (`KismetMathLibrary.MakeVector` _relativelocation_x _relativelocation_y (* FloorIndex (`self.GlobalOffset`))) (struct) false false (* (`KismetMathLibrary.Abs_Int` (- FloorIndex (`self.ActualLiftFloor`))) 2.5))
    (set `self.ActualLiftFloor` FloorIndex)))

(fn `UserConstructionScript`
  (locals (NewLocalVar :type "ChildActorComponent Object Reference"))
  (bind _playerstartref (`self.PlayerStartRef`))
  (bind (_returnvalue_x _returnvalue_y) (`KismetMathLibrary.BreakVector` (`self.K2_GetActorLocation` _playerstartref)))
  (`|ExecutionSequence`
    (:`then_0`
      ;[0.07292 0.07292 0.07292] Floor Manager
      (for _index (range (+ (`self.NumberOfFloor`) 1))
        ;;[0.07292 0.07292 0.07292] Shaft Body
        (`InstancedStaticMeshComponent.AddInstance` (`self.InstancedLiftShafBody`) (`KismetMathLibrary.MakeTransform` (`KismetMathLibrary.MakeVector` 0.0 0.0 (`KismetMathLibrary.Conv_IntToDouble` (* _index (`self.GlobalOffset`))))) false)
        ;;[0.07292 0.07292 0.07292] Shaft Door
        (`InstancedStaticMeshComponent.AddInstance` (`self.InstancedLiftShaftDoor`) (`KismetMathLibrary.MakeTransform` (`KismetMathLibrary.MakeVector` 0.0 0.0 (`KismetMathLibrary.Conv_IntToDouble` (* _index (`self.GlobalOffset`))))) false)
        ;;[0.07292 0.07292 0.07292] Floor
        (`InstancedStaticMeshComponent.AddInstance` (`self.InstancedLiftFloor`) (`KismetMathLibrary.MakeTransform` (`KismetMathLibrary.MakeVector` 0.0 0.0 (`KismetMathLibrary.Conv_IntToDouble` (* _index (`self.GlobalOffset`))))) false)
        (bind _returnvalue (`AddComponent|NODE_AddChildActorComponent-0` :`RelativeTransform` (`KismetMathLibrary.MakeTransform` (`KismetMathLibrary.MakeVector` (+ 0.0 -110.0) 0.0 (`KismetMathLibrary.Conv_IntToDouble` (+ (* _index (`self.GlobalOffset`)) 130))))))
        (bind _asbp_button (cast `/Game/MyBlueprints/BP_Button` (`ChildActorComponent.ChildActor` _returnvalue)))
        (set `/Game/MyBlueprints/BP_Button.FloorIndex` _index _asbp_button)))
    (:`then_1`
      ;[0.07292 0.07292 0.07292] Random Floor Lift Manager + Spawn Manager
      (set `self.ActualLiftFloor` (`KismetMathLibrary.RandomInteger` (`self.NumberOfFloor`)))
      (`SceneComponent.K2_SetRelativeTransform` (`self.LiftBase`) (`KismetMathLibrary.MakeTransform` (`KismetMathLibrary.MakeVector` 0.0 0.0 (`KismetMathLibrary.Conv_IntToDouble` (* 1000 (`self.ActualLiftFloor`))))) false false)
      (`self.K2_SetActorRelativeLocation` _playerstartref (`KismetMathLibrary.MakeVector` _returnvalue_x _returnvalue_y (+ 230.0 (`KismetMathLibrary.RandomInteger` (`self.NumberOfFloor`)))) false false))))