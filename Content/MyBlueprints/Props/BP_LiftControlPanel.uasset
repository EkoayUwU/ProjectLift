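; BP_LiftControlPanel is an interactable prop that gives the player a UI panel for a lift.
; On BeginPlay it creates a WBP_LiftControlPanel widget, adds it to the viewport and passes it the player controller, itself and its parent BP_Lift actor.
; Its Interaction event tells that widget to open.
; It expects to be a child actor of BP_Lift, since the widget setup stops if that cast fails.
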(event `self.ReceiveBeginPlay`
  (bind _returnvalue (`GameplayStatics.GetPlayerController` 0))
  ;[0.07292 0.07292 0.07292] Create ControlPanel Widget
  (bind _returnvalue_2 (`|CreateWidget` "/Game/MyBlueprints/Widgets/WBP_LiftControlPanel.WBP_LiftControlPanel_C" _returnvalue))
  (bind _output_get (set `self.WDLiftControlPanel` _returnvalue_2))
  (`UserWidget.AddToViewport` _returnvalue_2 0)
  (`UserWidget.AddToViewport` _output_get 0)
  (bind _asbp_lift (cast `/Game/MyBlueprints/Props/BP_Lift` (`self.GetParentActor`)))
  (`/Game/MyBlueprints/Widgets/WBP_LiftControlPanel.SetPanelRef` _output_get _returnvalue self _asbp_lift))

(event `/Game/MyBlueprints/BPI/BPI_Interact.Interaction`
  ;[0.07292 0.07292 0.07292] Open Control Panel Widget
  (`/Game/MyBlueprints/Widgets/WBP_LiftControlPanel.OpenWidget` (`self.WDLiftControlPanel`)))

(fn `UserConstructionScript`)