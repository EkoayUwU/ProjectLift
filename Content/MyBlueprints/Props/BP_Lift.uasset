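; Multi-floor lift prop that builds its own shaft and travels between floors when CallLift receives a floor index.
; The construction script stacks instanced shaft bodies, doors and floors, adds an indexed BP_Button per floor, randomizes the lift's starting floor and repositions a referenced player start.
; CallLift slides both doors to center with a timeline, moves the cabin over a distance-scaled time, then reverses the doors, or only reverses them on the current floor.
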(event `self.ReceiveBeginPlay`
  (bind _relativelocation_x (`KismetMathLibrary.BreakVector` (`SceneComponent.RelativeLocation` (`self.LiftDoorLeft`))))
  ;[0.07292 0.07292 0.07292] Init Door Pos
  (set `self.Relative Location DoorX` _relativelocation_x))

(event `Call Lift`
  (params (FloorIndex :type Integer))
  (bind _liftbase (`self.LiftBase`))
  (bind _liftdoorright (`self.LiftDoorRight`))
  (bind _liftdoorleft (`self.LiftDoorLeft`))
  (bind _relative_location_doorx (`self.Relative Location DoorX`))
  (bind (_relativelocation_x _relativelocation_y _relativelocation_z) (`KismetMathLibrary.BreakVector` (`SceneComponent.RelativeLocation` _liftdoorleft)))
  (bind (_relativelocation_x_2 _relativelocation_y_2 _relativelocation_z_2) (`KismetMathLibrary.BreakVector` (`SceneComponent.RelativeLocation` _liftdoorright)))
  (bind (_relativelocation_x_3 _relativelocation_y_3) (`KismetMathLibrary.BreakVector` (`SceneComponent.RelativeLocation` _liftbase)))
  ;[0.07292 0.07292 0.07292] Call Lift
  (if (!= FloorIndex (`self.ActualLiftFloor`))
    (bind (_direction _doormovement) (`Timeline|DoorMovement` :!via `PlayFromStart` :!label _label)
      (:`Update`
        (`|ExecutionSequence`
          (:`then_0`
            (`SceneComponent.K2_SetRelativeLocation` _liftdoorright (`KismetMathLibrary.MakeVector` (`KismetMathLibrary.Lerp` (* _relative_location_doorx -1.0) 0.0 _doormovement) _relativelocation_y_2 _relativelocation_z_2) false false))
          (:`then_1`
            (`SceneComponent.K2_SetRelativeLocation` _liftdoorleft (`KismetMathLibrary.MakeVector` (`KismetMathLibrary.Lerp` _relative_location_doorx 0.0 _doormovement) _relativelocation_y _relativelocation_z) false false))))
      (:`Finished`
        (if (!= FloorIndex (`self.ActualLiftFloor`))
          (set `self.BIsLiftMoving` true)
          (`KismetSystemLibrary.MoveComponentTo` _liftbase (`KismetMathLibrary.MakeVector` _relativelocation_x_3 _relativelocation_y_3 (* FloorIndex (`self.GlobalOffset`))) (struct) false false (* (`KismetMathLibrary.Abs_Int` (- FloorIndex (`self.ActualLiftFloor`))) 2.5))
          (set `self.BIsLiftMoving` false)
          (set `self.ActualLiftFloor` FloorIndex)
          (goto _label :!via `Reverse`))))
    (else
      (goto _label :!via `Reverse`))))

(fn `UserConstructionScript`
  (locals (NewLocalVar :type "ChildActorComponent Object Reference"))
  (bind _playerstartref (`self.PlayerStartRef`))
  (bind (_returnvalue_x _returnvalue_y) (`KismetMathLibrary.BreakVector` (`self.K2_GetActorLocation` _playerstartref)))
  (`|ExecutionSequence`
    (:`then_0`
      ;[0.07292 0.07292 0.07292] Floor Manager
      (for _index (range (+ (`self.NumberOfFloor`) 1))
        ;;[0.07292 0.07292 0.07292] Shaft Body
        (`InstancedStaticMeshComponent.AddInstance` (`self.InstancedLiftShafBody`) (`KismetMathLibrary.MakeTransform` (`KismetMathLibrary.MakeVector` 0.0 0.0 (`KismetMathLibrary.Conv_IntToDouble` (* _index (`self.GlobalOffset`))))) false)
        ;;[0.07292 0.07292 0.07292] Shaft Door
        (`InstancedStaticMeshComponent.AddInstance` (`self.InstancedLiftShaftDoor`) (`KismetMathLibrary.MakeTransform` (`KismetMathLibrary.MakeVector` 0.0 0.0 (`KismetMathLibrary.Conv_IntToDouble` (* _index (`self.GlobalOffset`))))) false)
        ;;[0.07292 0.07292 0.07292] Floor
        (`InstancedStaticMeshComponent.AddInstance` (`self.InstancedLiftFloor`) (`KismetMathLibrary.MakeTransform` (`KismetMathLibrary.MakeVector` 0.0 0.0 (`KismetMathLibrary.Conv_IntToDouble` (* _index (`self.GlobalOffset`))))) false)
        (bind _returnvalue (`AddComponent|NODE_AddChildActorComponent-0` :`RelativeTransform` (`KismetMathLibrary.MakeTransform` (`KismetMathLibrary.MakeVector` (+ 0.0 -110.0) 0.0 (`KismetMathLibrary.Conv_IntToDouble` (+ (* _index (`self.GlobalOffset`)) 130))))))
        (bind _asbp_button (cast `/Game/MyBlueprints/Props/BP_Button` (`ChildActorComponent.ChildActor` _returnvalue)))
        (set `/Game/MyBlueprints/Props/BP_Button.FloorIndex` _index _asbp_button)))
    (:`then_1`
      ;[0.07292 0.07292 0.07292] Random Floor Lift Manager + Spawn Manager
      (set `self.ActualLiftFloor` (`KismetMathLibrary.RandomInteger` (`self.NumberOfFloor`)))
      (`SceneComponent.K2_SetRelativeTransform` (`self.LiftBase`) (`KismetMathLibrary.MakeTransform` (`KismetMathLibrary.MakeVector` 0.0 0.0 (`KismetMathLibrary.Conv_IntToDouble` (* 1000 (`self.ActualLiftFloor`))))) false false)
      (`self.K2_SetActorRelativeLocation` _playerstartref (`KismetMathLibrary.MakeVector` _returnvalue_x _returnvalue_y (`KismetMathLibrary.Conv_IntToDouble` (+ (`KismetMathLibrary.RandomInteger` (`self.NumberOfFloor`)) 230))) false false))))